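; Player character Blueprint that handles rifle firing feedback and aim-down-sights zoom.
; Firing is gated by a CanFire flag and a cooldown timer, playing gun audio, a camera shake and paired arm and weapon montages, with the arm montage chosen by aim state.
; Starting or stopping aim stops the opposite mode's arm shooting montage and plays or reverses a timeline that drives camera FOV.
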(event `self.PlayFiringMontage`
  ;[1 1 1] Shooting
  (if (`self.GetCanFire`)
    (`self.SetCanFire` false)
    (`AudioComponent.Play` (`self.GunAudioComponent`) 0.0)
    (if (`self.GetIsAiming`)
      (`|PlayMontage` (`self.Mesh`) "/Game/FPS_Assault_Pack/Animations/Rifle/A_Arms_Rifle_Isight_Shoot01_Montage.A_Arms_Rifle_Isight_Shoot01_Montage"
        (:`then`
          _))
      (else
        (`|PlayMontage` (`self.Mesh`) "/Game/FPS_Assault_Pack/Animations/Rifle/A_Arms_Rifle_Shoot01_Montage.A_Arms_Rifle_Shoot01_Montage"
          (:`then`
            _))))
    (`KismetSystemLibrary.K2_SetTimerDelegate` (delegate `EnableShooting`) (`self.ShootingCooldown`))
    (`GameplayStatics.PlayWorldCameraShake` "/Game/MutantAI/Player/BP_CameraShake.BP_CameraShake_C" (`self.K2_GetActorLocation`) 1.0 500.0)
    (`|PlayMontage` (`self.Weapon`) "/Game/FPS_Assault_Pack/Animations/Rifle/A_Rifle_Shoot01_Montage.A_Rifle_Shoot01_Montage")))

(event `EnableShooting`
  ;[1 1 1] Shooting
  (`self.SetCanFire` true))

(event `self.StartAiming`
  ;[1 1 1] Aiming
  (`self.StopAnimMontage` "/Game/FPS_Assault_Pack/Animations/Rifle/A_Arms_Rifle_Shoot01_Montage.A_Arms_Rifle_Shoot01_Montage")
  (bind (_direction _fov) (`Timeline|AimingFOV` :!label _label)
    (:`Update`
      (`CameraComponent.SetFieldOfView` (`self.CameraComponent`) _fov))))

(event `self.StopAiming`
  ;[1 1 1] Aiming
  (`self.StopAnimMontage` "/Game/FPS_Assault_Pack/Animations/Rifle/A_Arms_Rifle_Isight_Shoot01_Montage.A_Arms_Rifle_Isight_Shoot01_Montage")
  (goto _label :!via `Reverse`))

(fn `UserConstructionScript`)