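; Mutant AI character Blueprint that plays the mutant's turn and attack animation montages on its mesh.
; Events start or stop the left or right turn montage according to a direction flag.
; The attack event sets IsPlayingAttackMontage, plays the attack montage and calls OnAttackMontageEnd only when playback completes, with no handling for interruption.
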(event `self.PlayTurnMontage`
  (params (bIsTurningLeft :type Boolean))
  (if bIsTurningLeft
    (`|PlayMontage` (`self.Mesh`) "/Game/Animations/Anim_Mutant_Turn_L_Montage.Anim_Mutant_Turn_L_Montage")
    (else
      (`|PlayMontage` (`self.Mesh`) "/Game/Animations/Anim_Mutant_Turn_R_Montage.Anim_Mutant_Turn_R_Montage"))))

(event `self.StopTurnMontage`
  (params (bIsTurningLeft :type Boolean))
  (if bIsTurningLeft
    (`self.StopAnimMontage` "/Game/Animations/Anim_Mutant_Turn_L_Montage.Anim_Mutant_Turn_L_Montage")
    (else
      (`self.StopAnimMontage` "/Game/Animations/Anim_Mutant_Turn_R_Montage.Anim_Mutant_Turn_R_Montage"))))

(event `self.PlayAttackMontage`
  (set `self.bIsPlayingAttackMontage` true)
  (`|PlayMontage` (`self.Mesh`) "/Game/Animations/Anim_Montage_Attack.Anim_Montage_Attack"
    (:`OnCompleted`
      (`self.OnAttackMontageEnd`))))

(fn `UserConstructionScript`)